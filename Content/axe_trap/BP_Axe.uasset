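; BP_Axe is an axe trap that swings and hurts the third-person character who enters its trigger box.
; Box overlap casts to BP_ThirdPersonCharacter and, unless that character's DeactivateAxe flag is set, plays a timeline.
; Each timeline update rotates the static mesh between two angles and subtracts health from the character, so damage accrues throughout playback without a blade hit check.
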(event OnComponentBeginOverlap(Box)
  (params (OverlappedComponent :type Primitive%20Component%20Object%20Reference) (OtherActor :type Actor%20Object%20Reference) (OtherComp :type Primitive%20Component%20Object%20Reference) (OtherBodyIndex :type Integer) (bFromSweep :type Boolean) (SweepResult :type Hit%20Result%20Structure%20%28by%20ref%29))
  (bind _asbp_third_person_character (Utilities|Casting|CastToBP_ThirdPersonCharacter OtherActor))
  (if (not (Variables|/Game/BP_ThirdPersonCharacter.BP_ThirdPersonCharacter_C|GetDeactivateAxe _asbp_third_person_character))
    (bind _newtrack_0 (Timeline|Timeline Play)
      (:Update
        (Transformation|SetWorldRotation (Variables|Default|GetStaticMesh) (.rotation (Math|Transform|Lerp(Transform) (Math|Transform|MakeTransform "0, 0, 0" "-80.000000,0.000000,180.000000" "1.000000,1.000000,1.000000") (Math|Transform|MakeTransform "0, 0, 0" "80.000000,0.000000,180.000000" "1.000000,1.000000,1.000000") _newtrack_0)) false false)
        (Variables|/Game/BP_ThirdPersonCharacter.BP_ThirdPersonCharacter_C|SetCurrentHealth _asbp_third_person_character (- (Variables|/Game/BP_ThirdPersonCharacter.BP_ThirdPersonCharacter_C|GetCurrentHealth _asbp_third_person_character) 5))))))

(event EventBeginPlay)

(event Collision|EventActorBeginOverlap
  (params (OtherActor :type Actor%20Object%20Reference)))

(event EventTick
  (params (DeltaSeconds :type Float%20%28single-precision%29)))

(fn ConstructionScript)