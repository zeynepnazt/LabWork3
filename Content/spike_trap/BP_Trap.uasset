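; Spike trap actor that damages BP_ThirdPersonCharacter when it enters the Box trigger, unless that character's DeactivateTrap flag is set.
; On overlap, a timeline lerps the Torn component upward in relative space.
; Every timeline update also subtracts one point from the character's CurrentHealth, so damage scales with update count.
; When health reaches zero or below, DestroyActor removes the trap itself, not the character.
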(event OnComponentBeginOverlap(Box)
  (params (OverlappedComponent :type Primitive%20Component%20Object%20Reference) (OtherActor :type Actor%20Object%20Reference) (OtherComp :type Primitive%20Component%20Object%20Reference) (OtherBodyIndex :type Integer) (bFromSweep :type Boolean) (SweepResult :type Hit%20Result%20Structure%20%28by%20ref%29))
  (bind _asbp_third_person_character (Utilities|Casting|CastToBP_ThirdPersonCharacter OtherActor))
  (if (not (Variables|/Game/BP_ThirdPersonCharacter.BP_ThirdPersonCharacter_C|GetDeactivateTrap _asbp_third_person_character))
    (bind _newtrack_0 (Timeline|Timeline Play)
      (:Update
        (Transformation|SetRelativeLocation (Variables|Default|GetTorn) (Math|Vector|Lerp(Vector) "250.000000,230.000000,-90.000000" "250.000000,230.000000,0.000000" _newtrack_0) false false)
        (bind _output_get (Variables|/Game/BP_ThirdPersonCharacter.BP_ThirdPersonCharacter_C|SetCurrentHealth _asbp_third_person_character (- (Variables|/Game/BP_ThirdPersonCharacter.BP_ThirdPersonCharacter_C|GetCurrentHealth _asbp_third_person_character) 1)))
        (if (<= _output_get 0)
          (Actor|DestroyActor))))))

(event EventBeginPlay)

(event Collision|EventActorBeginOverlap
  (params (OtherActor :type Actor%20Object%20Reference)))

(event EventTick
  (params (DeltaSeconds :type Float%20%28single-precision%29)))

(fn ConstructionScript)