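; BP_SlidingDoor1 is a key-locked sliding door that opens on an Interact event.
; Interact compares the Keys value on the third-person game mode with the door's KeyNumber, requiring an exact match, and prints a message otherwise.
; On a match, the Door_Rotate timeline lerps the door mesh's relative location from start to finish, despite its rotation-based name.
; The construction script applies the configurable Material to the door mesh.
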(event EventInteract
  (if (== (Variables|/Game/ThirdPerson/Blueprints/BP_ThirdPersonGameMode.BP_ThirdPersonGameMode_C|GetKeys (Variables|Default|GetAs%20Bp_ThirdPersonGameMode)) (Variables|Default|GetKeyNumber))
    (bind _newtrack_0 (Timeline|Door_Rotate Play)
      (:Update
        (Transformation|SetRelativeLocation (Variables|Default|GetSM_Door) (Math|Vector|Lerp(Vector) (Variables|Default|GetStartLocation) (Variables|Default|GetFinishLocation) _newtrack_0) false false)))
    (else
      (Development|PrintString "You don't have to correct keys"))))

(fn ConstructionScript
  (Rendering|Material|SetMaterial (Variables|Default|GetSM_Door) 0 (Variables|Default|GetMaterial)))