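; BP_Keys is an interactable key pickup that records which key was taken in BP_ThirdPersonGameMode.
; It caches the game mode on BeginPlay, and Interact overwrites that mode's Keys value with its KeyNumber, prints an acquired message using the Names lookup, and destroys the actor.
; The construction script applies the Material variable to the Keys component, so each instance can have its own look.
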(event EventBeginPlay
  (bind _asbp_third_person_game_mode (Utilities|Casting|CastToBP_ThirdPersonGameMode (Game|GetGameMode)))
  (Variables|Default|SetAs%20BP%20Third%20Person%20Game%20Mode _asbp_third_person_game_mode))

(event EventInteract
  (bind _output_get (Variables|/Game/ThirdPerson/Blueprints/BP_ThirdPersonGameMode.BP_ThirdPersonGameMode_C|SetKeys (Variables|Default|GetAs%20BP%20Third%20Person%20Game%20Mode) (Variables|Default|GetKeyNumber)))
  (Development|PrintString (Utilities|String|Append "Key" (Utilities|Array|Get(acopy) (Variables|Default|GetNames) _output_get) "Acquired"))
  (Actor|DestroyActor))

(fn ConstructionScript
  (Rendering|Material|SetMaterial (Variables|Default|GetKeys) 0 (Variables|Default|GetMaterial)))